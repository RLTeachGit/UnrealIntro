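; A key pickup Blueprint that gives the player a door key of a configured type when picked up.
; It extends a parent pickup's PlayerPickup event, passing its DoorKey value to the player's AddKey.
; The construction script builds a dynamic material on the mesh and sets its Glow colour from a colour array indexed by the key enum, so the colour also shows in the editor.
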(event `self.PlayerPickup`
  (params (Player :type "/Game/ThirdPersonBP/Blueprints/MyCharacter Object Reference"))
  ;[1 1 1] Handle player key pickup
  (`parent.PlayerPickup` Player)
  (`/Game/ThirdPersonBP/Blueprints/MyCharacter.AddKey` Player (`self.DoorKey`)))

(fn `UserConstructionScript`
  ;[1 1 1] Constructor also runs in Editor
  (`parent.UserConstructionScript`)
  ;[1 1 1] Create a Dynamic Material and set its colour based on Key Colour
  (bind _returnvalue (`PrimitiveComponent.CreateDynamicMaterialInstance` (`self.StaticMeshComponent`) 0 "/Game/Door/KeyMaterial.KeyMaterial" "None"))
  (bind _output_get (set `self.GlowMaterial` _returnvalue))
  (`MaterialInstanceDynamic.SetVectorParameterValue` _output_get "Glow" (`|GetArrayItem` (`self.KeyColours`) (`KismetMathLibrary.Conv_ByteToInt` (`self.DoorKey`)))))