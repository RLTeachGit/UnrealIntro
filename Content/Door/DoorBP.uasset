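; Door Blueprint that swings its Door component open around yaw by an angle passed to the OpenDoor event.
; A Sweep timeline scales that angle by its curve value each update to set the relative rotation.
; An IsBusy flag ignores new requests during a swing, and ResetDoor clears it and rewinds the timeline when the sweep finishes.
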(event `OpenDoor`
  (params (OpenAngle :type "Float (double-precision)"))
  ;[1 1 1] Open door event
  (if (not (`self.isBusy`))
    (set `self.isBusy` true)
    (set `self.OpenAngle` OpenAngle)
    ;[1 1 1] Open door by rotating it
    (bind (_direction _sweepval) (`Timeline|Sweep` :!label _label)
      (:`Update`
        (`SceneComponent.K2_SetRelativeRotation` (`self.Door`) (`KismetMathLibrary.MakeRotator` 0.0 0.0 (* _sweepval (`self.OpenAngle`))) false false))
      (:`Finished`
        (`self.ResetDoor`)))))

(event `ResetDoor`
  ;[1 1 1] Reset door
  (set `self.isBusy` false)
  (goto _label :!via `SetNewTime`))

(fn `UserConstructionScript`)